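; Base machine actor for a production chain worked by agents, holding a stock that can decay on a looping timer.
; Working it consumes stock, feeds the produced amount into its connected machine and, like decay, notifies the GameMode.
; A handshake reserves it for one agent until stopped or that agent leaves the collider.
; Tick refreshes the stock text and a dynamic-material colour band, which is also exposed as a perception state.
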(event `self.ReceiveTick`
  (params (DeltaSeconds :type "Float (single-precision)"))
  ;[1 1 1] Display machine's stock status
  (`|ExecutionSequence`
    (:`then_0`
      (if (not (`|EnumEquality` (`self.ConsumedElement`) "NewEnumerator11"))
        (`self.displayMachineInfo`)
        (else
          (`TextRenderComponent.SetText` ""))))
    (:`then_1`
      (`self.MachineMaterialColor`))))

(event `self.ReceiveBeginPlay`
  (bind _returnvalue (`PrimitiveComponent.CreateDynamicMaterialInstance` (`self.MachineMesh`) 0 null))
  (set `self.StaticMeshMaterial` _returnvalue)
  ;[1 1 1] Cause Decay
  (if (`self.bHasDecay`)
    (`KismetSystemLibrary.K2_SetTimer` self "DecayFunction" (`self.DecayTime`) true)))

(event `self.SphereCollider.OnComponentBeginOverlap`
  (params (OtherActor :type "Actor Object Reference") (OtherComp :type "PrimitiveComponent Object Reference") (OtherBodyIndex :type Integer) (bFromSweep :type Boolean) (SweepResult :type "EngineTypes.HitResult Structure (by ref)"))
  ;[1 1 1] Work Machine
)

(event `self.InteractWithMachine`
  (params (Agent :type "Actor Object Reference"))
  ;[1 1 1] Work Machine
  (`self.WorkMachine` Agent))

(event `self.SphereCollider.OnComponentEndOverlap`
  (params (OtherActor :type "Actor Object Reference") (OtherComp :type "PrimitiveComponent Object Reference") (OtherBodyIndex :type Integer))
  ;[1 1 1] Stop Work Machine
  (`self.ProcessColliderOverlapEnd` OtherActor))

(event `self.StopHandShake`
  (params (Agent :type "Actor Object Reference"))
  ;[1 1 1] Stop Work Machine
  (`self.FinishHandShake` Agent))

(fn `CanWork?`
  (params (Agent :type "Actor Object Reference"))
  (returns (CanWork :type Boolean))
  ;[1 1 1] CheckIfAnyoneIsWorking
  (if (`self.bIsWorking`)
    ;[1 1 1] CheckIfAgentIsAlreadyWorking
    (if (== Agent (`self.WorkingAgent`))
      (set `self.bCanWork` true :!label _label)
      (else
        (set `self.bCanWork` false)))
    (else
      (set `self.bIsWorking` true)
      ;[1 0.2352 0.1778] TellingTheMachineWhoIsWorking
      (bind _output_get (set `self.WorkingAgent` Agent))
      ;[1 0.1599 0.1695] TellingTheAgentBody
      (message `/Game/OurContent/Blueprints/BPI_Gameplay/BPI_AI_Character.SetIsWorking` _output_get true)
      (goto _label)))
  (return (`self.bCanWork`)))

(fn `DecayFunction`
  (bind _stock (`self.Stock`))
  (bind _returnvalue (`KismetSystemLibrary.GetDisplayName` self))
  (`|ExecutionSequence`
    (:`then_0`
      ;[0.6539 0.6464 1] Machine Stock Decay Effect
      (if (> _stock 0)
        (set `self.Stock` (- _stock (`self.DecayAmount`)))
        ;[1 1 1] Debugging
        (if (== _returnvalue (`KismetSystemLibrary.GetDisplayName` null))
          (`KismetSystemLibrary.PrintString` (`KismetStringLibrary.Concat_StrStr` (`KismetStringLibrary.Concat_StrStr` _returnvalue " Has stock value: ") (`KismetStringLibrary.Conv_IntToString` _stock))))))
    (:`then_1`
      ;[0.6141 1 0.622] Update Game Mode
      (message `/Game/OurContent/Blueprints/BPI_Gameplay/BPI_Game_Mode.CauseDecay` (`GameplayStatics.GetGameMode`) (`self.MachineType`) (`self.DecayAmount`)))))

(fn `displayMachineInfo`
  ;[1 1 1] Display machine's stock status
  (`TextRenderComponent.SetText` (`KismetStringLibrary.Concat_StrStr` (`self.StockString`) (`KismetStringLibrary.Conv_IntToString` (`self.Stock`)))))

(fn `FinishHandShake`
  (params (Agent :type "Actor Object Reference"))
  (bind _output_get (set `self.bIsWorking` false))
  ;[1 0.1599 0.1695] TellingTheAgentBody
  (message `/Game/OurContent/Blueprints/BPI_Gameplay/BPI_AI_Character.SetIsWorking` Agent _output_get))

(fn `GetAmmountOfStock`
  (returns (StockAmmount :type Integer))
  (return (`self.Stock`)))

(fn `getConsumedElement`
  (returns (ConsumedElement :type "/Game/OurContent/Enumerations/E_MachineElements Enum") (Stock :type Integer))
  (return (`self.ConsumedElement`) (`self.Stock`)))

(fn `getMachineColorPerception`
  (returns (MachineColor :type Name))
  (return (`self.MachineColorState`)))

(fn `getProducedElement`
  (returns (NewParam :type Boolean))
  (return false))

(fn `IsBeingUsed?`
  (params (Agent :type "Actor Object Reference"))
  (returns (IsUsed :type Boolean))
  (if (`self.bIsWorking`)
    (if (== Agent (`self.WorkingAgent`))
      (set `self.bCanAgentUse` false :!label _label)
      (else
        (set `self.bCanAgentUse` true)))
    (else
      (goto _label)))
  (return (`self.bCanAgentUse`)))

(fn `MachineConnection`
  (params (`Produced Ammount` :type Integer :default 0))
  ;[1 1 1] Target Machine Stock Update
  (set `self.Stock` (+ (`self.Stock`) `Produced Ammount`)))

(fn `MachineMaterialColor`
  (bind _stock (`self.Stock`))
  (if (== _stock 0)
    (set `self.MachineColorState` "Black")
    (`MaterialInstanceDynamic.SetScalarParameterValue` (`self.StaticMeshMaterial`) "PercentageOfInterpolate" 1.0)
    (`MaterialInstanceDynamic.SetVectorParameterValue` (`self.StaticMeshMaterial`) "StockEffectColor" (make `Object.LinearColor` 0.0))
    (elif (and (> _stock 0) (< _stock 20))
      (set `self.MachineColorState` "Red")
      (`MaterialInstanceDynamic.SetScalarParameterValue` (`self.StaticMeshMaterial`) "PercentageOfInterpolate" 0.8)
      (`MaterialInstanceDynamic.SetVectorParameterValue` (`self.StaticMeshMaterial`) "StockEffectColor" (make `Object.LinearColor` 1.0))
      (elif (and (>= _stock 20) (< _stock 40))
        (set `self.MachineColorState` "Yellow")
        (`MaterialInstanceDynamic.SetScalarParameterValue` (`self.StaticMeshMaterial`) "PercentageOfInterpolate" 0.5)
        (`MaterialInstanceDynamic.SetVectorParameterValue` (`self.StaticMeshMaterial`) "StockEffectColor" (make `Object.LinearColor` 1.0 1.0))
        (else
          (set `self.MachineColorState` "Green")
          (`MaterialInstanceDynamic.SetScalarParameterValue` (`self.StaticMeshMaterial`) "PercentageOfInterpolate" 0.0))))))

(fn `ProcessColliderOverlapBegin`
  (params (AgentCollider :type "Actor Object Reference"))
  (if (`self.bCanWork`)
    (set `self.WorkingAgent` AgentCollider)
    (set `self.bCanWork` false)
    (`KismetSystemLibrary.K2_SetTimer` self "WorkMachine" (`self.WorkSpeed`) true)))

(fn `ProcessColliderOverlapEnd`
  (params (`Agent Collider` :type "Actor Object Reference"))
  (if (== `Agent Collider` (`self.WorkingAgent`))
    (`self.FinishHandShake` `Agent Collider`)))

(fn `UserConstructionScript`
  (bind _arrow (`self.Arrow`))
  (`StaticMeshComponent.SetStaticMesh` (`self.MachineMesh`) (`self.StaticMeshToDisplay`))
  (if (not (== (`self.ConnectedMachine`) null))
    (`SceneComponent.SetVisibility` _arrow true false)
    (`SceneComponent.K2_SetWorldRotation` _arrow (`KismetMathLibrary.FindLookAtRotation` (`self.K2_GetActorLocation`) (`self.K2_GetActorLocation` (`self.ConnectedMachine`))) false)))

(fn `WorkMachine`
  (params (Agent :type "Actor Object Reference"))
  (bind _stock (`self.Stock`))
  (bind _consumedamount (`self.ConsumedAmount`))
  (bind _producedamount (`self.ProducedAmount`))
  (`|ExecutionSequence`
    (:`then_0`
      ;[0.628 1 0.6668] Update GameMode
      (message `/Game/OurContent/Blueprints/BPI_Gameplay/BPI_Game_Mode.WorkMachine` (`GameplayStatics.GetGameMode`) (`self.MachineType`) _consumedamount _producedamount))
    (:`then_1`
      ;[0.4975 0.5072 1] Update Machine Stocks
      (if (> _stock 0)
        (set `self.Stock` (- _stock _consumedamount))
        (`self.MachineConnection` (`self.ConnectedMachine`) _producedamount)))))