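; BP_Machine_Child_Mapas is a child machine Blueprint, named for maps, that handles an agent working it.
; WorkMachine first reports its machine type and consumed and produced amounts to the game mode.
; It then passes the produced amount to its connected machine and applies a hunger debuff to the agent.
; The construction script only calls the parent's, and the other events are disabled stubs.
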(event `self.ReceiveBeginPlay`)

(event `self.ReceiveActorBeginOverlap`
  (params (OtherActor :type "Actor Object Reference")))

(event `self.ReceiveTick`
  (params (DeltaSeconds :type "Float (single-precision)")))

(event `self.WorkMachine`
  (params (Agent :type "Actor Object Reference"))
  (bind _producedamount (`self.ProducedAmount`))
  (`|ExecutionSequence`
    (:`then_0`
      (message `/Game/OurContent/Blueprints/BPI_Gameplay/BPI_Game_Mode.WorkMachine` (`GameplayStatics.GetGameMode`) (`self.MachineType`) (`self.ConsumedAmount`) _producedamount))
    (:`then_1`
      (`self.MachineConnection` (`self.ConnectedMachine`) _producedamount)
      (message `/Game/OurContent/Blueprints/BPI_Gameplay/BPI_AI_Character.DoHungerDeBuff` Agent (`self.HungerDebuff`)))))

(fn `UserConstructionScript`
  (`parent.UserConstructionScript`))