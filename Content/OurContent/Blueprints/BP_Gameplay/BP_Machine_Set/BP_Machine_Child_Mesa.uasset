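; BP_Machine_Child_Mesa is a machine child Blueprint, likely a table, that serves plates to agents.
; On WorkMachine it reports its machine type with consumed and produced amounts to the GameMode.
; If Stock is above zero, it then subtracts the consumed amount and messages the agent to give it a plate to eat.
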(event `self.ReceiveBeginPlay`)

(event `self.ReceiveActorBeginOverlap`
  (params (OtherActor :type "Actor Object Reference")))

(event `self.ReceiveTick`
  (params (DeltaSeconds :type "Float (single-precision)")))

(event `self.FinishHandShake`
  (params (Agent :type "Actor Object Reference")))

(event `self.WorkMachine`
  (params (Agent :type "Actor Object Reference"))
  (bind _stock (`self.Stock`))
  (bind _consumedamount (`self.ConsumedAmount`))
  (`|ExecutionSequence`
    (:`then_0`
      ;[0.628 1 0.6668] Update GameMode
      (message `/Game/OurContent/Blueprints/BPI_Gameplay/BPI_Game_Mode.WorkMachine` (`GameplayStatics.GetGameMode`) (`self.MachineType`) _consumedamount (`self.ProducedAmount`)))
    (:`then_1`
      ;[0.4975 0.5072 1] UpdatePlateNumber
      (if (> _stock 0)
        (set `self.Stock` (- _stock _consumedamount))
        (message `/Game/OurContent/Blueprints/BPI_Gameplay/BPI_AI_Character.GivePlateToEat` Agent)))))

(fn `UserConstructionScript`
  (`parent.UserConstructionScript`))