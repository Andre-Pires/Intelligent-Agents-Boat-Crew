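; BP_Room is a room actor for exploration that tracks which points and doors belong to a room.
; When an actor overlaps its Box, it sends that actor a GiveRoomNameMessage carrying a reference to itself.
; CheckIfExplored reports the room explored only if the supplied agent lists contain every one of its Points and Doors.
; GetDoors exposes the room's door list to callers.
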(event OnComponentBeginOverlap(Box)
  (params (OtherActor :type Actor%20Object%20Reference) (OtherComp :type Primitive%20Component%20Object%20Reference) (OtherBodyIndex :type Integer) (bFromSweep :type Boolean) (SweepResult :type Hit%20Result%20Structure%20%28by%20ref%29))
  (Class|BPIAICharacter|GiveRoomName(Message) OtherActor self))

(event EventBeginPlay)

(event EventActorBeginOverlap
  (params (OtherActor :type Actor%20Object%20Reference)))

(event EventTick
  (params (DeltaSeconds :type Float%20%28single-precision%29)))

(fn ConstructionScript)

(fn CheckifExplored
  (params (agentsPoints :type Array%20of%20Actor%20Object%20References) (agentsDoors :type Array%20of%20Actor%20Object%20References))
  (LocalVariables|SetisExplored true)
  (Utilities|FlowControl|Sequence
    (:then_0
      (bind _array_element (Utilities|Array|ForEachLoopwithBreak (Variables|Default|GetPoints) :!label _label)
        (:LoopBody
          (if (not (Utilities|Array|ContainsItem agentsPoints _array_element))
            (LocalVariables|SetisExplored false)
            (goto _label Break)))))
    (:then_1
      (bind _array_element_2 (Utilities|Array|ForEachLoopwithBreak (Variables|Default|GetDoors) :!label _label_2)
        (:LoopBody
          (if (not (Utilities|Array|ContainsItem agentsDoors _array_element_2))
            (LocalVariables|SetisExplored false)
            (goto _label_2 Break)))))
    (:then_2
      (return (LocalVariables|GetisExplored)))))

(fn GetDoors
  (return (Variables|Default|GetDoors)))