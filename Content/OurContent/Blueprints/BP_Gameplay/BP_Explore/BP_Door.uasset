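; BP_Door is an exploration door actor that computes a destination point on the opposite side of itself from a given character.
; The construction script applies a configurable static mesh to MachineMesh.
; GetTheOtherSide compares world Y positions and returns the door's location plus the RightSide or LeftSide offset.
; The side test ignores door rotation, and the file itself does not move the character.
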(fn ConstructionScript
  (Components|StaticMesh|SetStaticMesh (Variables|Default|GetMachineMesh) (Variables|Default|GetStaticMeshToDisplay)))

(fn GettheOtherSide
  (params (Character :type Actor%20Object%20Reference))
  (bind _returnvalue (Transformation|GetActorLocation))
  (if (< (.Y (Math|Vector|BreakVector (Transformation|GetActorLocation Character))) (.Y (Math|Vector|BreakVector (Transformation|GetActorLocation))))
    (LocalVariables|SetsideToReturn (+ _returnvalue (Variables|Default|GetrightSide)))
    (else
      (LocalVariables|SetsideToReturn (+ _returnvalue (Variables|Default|GetleftSide)))))
  (return (LocalVariables|GetsideToReturn)))