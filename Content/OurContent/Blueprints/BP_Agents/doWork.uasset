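; Behavior tree task in which an agent completes a handshake with its target machine, depending on that machine's stock.
; It reads the TargetToFollow blackboard actor and queries its stock through message calls.
; With stock, it sends an interact message for SelfActor, waits briefly and succeeds.
; Without stock, it sends a stop-handshake message, clears TargetToFollow and fails.
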(event `self.ReceiveExecute`
  (params (OwnerActor :type "Actor Object Reference"))
  (bind _returnvalue (`BTFunctionLibrary.GetBlackboardValueAsActor` (`self.SelfActor`)))
  (bind _returnvalue_2 (`BTFunctionLibrary.GetBlackboardValueAsActor` (`self.TargetToFollow`)))
  (bind _stockammount (message `/Game/OurContent/Blueprints/BPI_Gameplay/BPI_Interactable.GetAmmountOfStock` _returnvalue_2))
  (if (> _stockammount 0)
    ;[1 1 1] Continue handshake, there is enough stock
    (message `/Game/OurContent/Blueprints/BPI_Gameplay/BPI_Interactable.InteractWithMachine` _returnvalue_2 _returnvalue)
    (`KismetSystemLibrary.Delay` 0.5)
    (`self.FinishExecute` true)
    (else
      ;[1 1 1] Stop handshake, there is no stock
      (message `/Game/OurContent/Blueprints/BPI_Gameplay/BPI_Interactable.StopHandShake` _returnvalue_2 _returnvalue)
      (`BTFunctionLibrary.SetBlackboardValueAsObject` (`self.TargetToFollow`))
      (`self.FinishExecute` false))))