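; Behavior tree decorator that randomly decides, roughly 40% of the time, whether a follower AI should head for a nearby teleporter.
; On a successful roll, it sphere-traces around the pawn for Teleporter-tagged actors, ignoring AI characters, then line-traces to confirm line of sight.
; A visible teleporter's location goes into the RandomLocation blackboard key and the check passes; a blocked one zeroes the key.
; Both traces draw debug shapes.
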(fn `PerformConditionCheck`
  (params (OwnerActor :type "Actor Object Reference"))
  (returns (ReturnValue :type Boolean))
  (bind _randomlocation (`self.RandomLocation`))
  (bind _returnvalue (`Actor.K2_GetActorLocation` (`Controller.K2_GetPawn` (`self.AI_CON_Ref`))))
  (if (not (!= (`self.AI_CON_Ref`) null))
    (bind _asfollower_ai_con (cast `/Game/OurContent/Blueprints/BP_Agents/Follower_AI_CON` OwnerActor))
    (set `self.AI_CON_Ref` _asfollower_ai_con))
  (bind _output_get (set `self.willTeleport` (< (`KismetMathLibrary.RandomIntegerInRange` 0 100) 40)))
  (if _output_get
    (bind _outactors (`GameplayStatics.GetAllActorsOfClass` "/Game/OurContent/Blueprints/BP_Agents/AI_Character.AI_Character_C"))
    (set `self.MyLocation` _returnvalue)
    (bind _outhits (`KismetSystemLibrary.SphereTraceMultiForObjects` _returnvalue (+ _returnvalue (0.0 0.0 15.0)) 1500.0 (`|MakeArray` "ObjectTypeQuery2" :!type "EngineTypes.EObjectTypeQuery Enum") false _outactors "ForDuration"))
    (for _array_element _outhits
      (bind (_bblockinghit _time _location _normal _impactpoint _impactnormal _physmat _hitactor) (`GameplayStatics.BreakHitResult` _array_element))
      ;[1 1 1] Test if actor found teleport
      (if (`Actor.ActorHasTag` _hitactor (`self.Teleporter`))
        (bind _outhit (`KismetSystemLibrary.LineTraceSingle` (`self.MyLocation`) (`Actor.K2_GetActorLocation` _hitactor) "TraceTypeQuery2" false _outactors "ForDuration"))
        (bind (_bblockinghit_2 _time_2 _location_2 _normal_2 _impactpoint_2 _impactnormal_2 _physmat_2 _hitactor_2) (`GameplayStatics.BreakHitResult` _outhit))
        (if (== _hitactor_2 _hitactor)
          (`BTFunctionLibrary.SetBlackboardValueAsVector` _randomlocation (`Actor.K2_GetActorLocation` _hitactor_2))
          (return (`self.willTeleport`))
          (else
            (`BTFunctionLibrary.SetBlackboardValueAsVector` _randomlocation)))))
    (else
      (return (`self.willTeleport`)))))