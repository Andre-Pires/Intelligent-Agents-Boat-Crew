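; Behavior tree node that turns an AI agent's perceptions into Blackboard beliefs each tick.
; It caches the Follower_AI_CON controller, sets SelfActor, then runs sleepy, hungry and machine-vision rules.
; Sleepy and hungry flags both compare the character's Hunger to ThresholdHunger.
; The vision rule clears TargetToFollow and sphere-traces around the pawn, collecting machines not in use into a temporary array without writing them to the Blackboard.
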(event `ReceiveTick_Copy_Copy`
  (params (OwnerActor :type "Actor Object Reference") (DeltaSeconds :type "Float (double-precision)" :default 0.0))
  (if (not (!= (`self.AI_CON_Ref`) null))
    ;[1 1 1] Define AICON if not defined
    (bind _asfollower_ai_con (cast `/Game/OurContent/Blueprints/BP_Agents/Follower_AI_CON` null))
    (set `self.AI_CON_Ref` _asfollower_ai_con))
  (`BTFunctionLibrary.SetBlackboardValueAsObject` (`self.SelfActor`) (`Controller.K2_GetPawn` (`self.AI_CON_Ref`)))
  ;[0.81 0.799 0.4571] Perception Rules
  (`self.isSleepyPerception`)
  (`self.isHungryPerception`)
  (`self.MachinesInVisionPerception`))

(fn `isHungryPerception`
  (bind _asai_character (cast `/Game/OurContent/Blueprints/BP_Agents/AI_Character` (`BTFunctionLibrary.GetBlackboardValueAsActor` (`self.SelfActor`))))
  (`BTFunctionLibrary.SetBlackboardValueAsBool` (`self.bIsHungryPerception`) (<= (`/Game/OurContent/Blueprints/BP_Agents/AI_Character.hunger` _asai_character) (`self.ThresholdHunger`))))

(fn `isSleepyPerception`
  (bind _asai_character (cast `/Game/OurContent/Blueprints/BP_Agents/AI_Character` (`BTFunctionLibrary.GetBlackboardValueAsActor` (`self.SelfActor`))))
  (`BTFunctionLibrary.SetBlackboardValueAsBool` (`self.bIsSleepyPerception`) (<= (`/Game/OurContent/Blueprints/BP_Agents/AI_Character.hunger` _asai_character) (`self.ThresholdHunger`))))

(fn `MachinesInVisionPerception`
  (bind _returnvalue (`Controller.K2_GetPawn` (`self.AI_CON_Ref`)))
  (bind _returnvalue_2 (`Actor.K2_GetActorLocation` _returnvalue))
  (`BTFunctionLibrary.SetBlackboardValueAsObject` (`self.TargetToFollow`))
  (bind _outactors (`GameplayStatics.GetAllActorsOfClass` "/Game/OurContent/Blueprints/BP_Agents/AI_Character.AI_Character_C"))
  (set `self.MyLocation` _returnvalue_2)
  (bind _outhits (`KismetSystemLibrary.SphereTraceMultiForObjects` _returnvalue_2 (+ _returnvalue_2 (0.0 0.0 15.0)) 1500.0 (`|MakeArray` "ObjectTypeQuery2" :!type "EngineTypes.EObjectTypeQuery Enum") false _outactors))
  (for _array_element _outhits
    (bind (_bblockinghit _time _location _normal _impactpoint _impactnormal _physmat _hitactor) (`GameplayStatics.BreakHitResult` _array_element))
    ;[1 1 1] Test If Actor is working or has empty machine to work
    (bind _isused (message `/Game/OurContent/Blueprints/BPI_Gameplay/BPI_Interactable.IsBeingUsed?` _hitactor _returnvalue))
    (if (not _isused)
      (`KismetArrayLibrary.Array_Add` (`self.TempWorkableMachineArray`) _hitactor))))