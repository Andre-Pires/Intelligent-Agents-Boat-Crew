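; RapidMoveTo is a Behavior Tree task that moves an AI agent's pawn to the actor held in the TargetToFollow blackboard key.
; It casts and caches the owning AIController on first use, then reissues AIMoveTo on every tick rather than once at execution.
; The task finishes successfully when a move reaches the acceptance radius, and has no handling for failed moves.
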(event `self.ReceiveTick`
  (params (OwnerActor :type "Actor Object Reference") (DeltaSeconds :type "Float (single-precision)"))
  (if (not (!= (`self.AI_CON_Ref`) null))
    (bind _asaicontroller (cast `AIController` OwnerActor))
    (set `self.AI_CON_Ref` _asaicontroller))
  (`|AIMoveTo` (`Controller.K2_GetPawn` (`self.AI_CON_Ref`)) (0.0 0.0 0.0) (`BTFunctionLibrary.GetBlackboardValueAsActor` (`self.TargetToFollow`)) 100.0 true
    (:`OnSuccess`
      (`self.FinishExecute` true))))