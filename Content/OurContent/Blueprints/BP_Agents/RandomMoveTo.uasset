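; Behavior tree task that sends an AI-controlled pawn to a random location.
; It casts the owner to AIController on first execution and caches the reference for later runs.
; The destination comes from a large radius around a fixed world X/Y origin at the pawn's current height, rather than around the pawn.
; The task finishes only when AIMoveTo succeeds; a failed move or cast never calls FinishExecute.
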(event `self.ReceiveExecute`
  (params (OwnerActor :type "Actor Object Reference"))
  (bind _returnvalue (`Controller.K2_GetPawn` (`self.AI_CON_Ref`)))
  (if (not (!= (`self.AI_CON_Ref`) null))
    (bind _asaicontroller (cast `AIController` OwnerActor))
    (set `self.AI_CON_Ref` _asaicontroller))
  (`|AIMoveTo` _returnvalue (`NavigationSystem.GetRandomPointInRadius` (`KismetMathLibrary.MakeVector` -265.0 0.0 (.z (`Actor.K2_GetActorLocation` _returnvalue))) 50000.0) null 100.0 true
    (:`OnSuccess`
      (`self.FinishExecute` true))))