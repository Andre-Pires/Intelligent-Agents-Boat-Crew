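; Behavior tree task that establishes a work handshake between an agent and the actor in its TargetToFollow blackboard key.
; For a Machine-tagged target, it calls CanWorkMessage with SelfActor, stores the answer in BIsWorking, clears the target on refusal and finishes with that result.
; Other targets never reach FinishExecute.
; Table and Bed tag checks exist but are disconnected from execution.
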(event `self.ReceiveExecute`
  (params (OwnerActor :type "Actor Object Reference"))
  (bind _returnvalue (`BTFunctionLibrary.GetBlackboardValueAsActor` (`self.TargetToFollow`)))
  ;[1 1 1] Work
  (if (`Actor.ActorHasTag` _returnvalue "Machine")
    ;[0.7369 1 0.9617] MachineCheck
    (bind _canwork (message `/Game/OurContent/Blueprints/BPI_Gameplay/BPI_Interactable.CanWork?` _returnvalue (`BTFunctionLibrary.GetBlackboardValueAsActor` (`self.SelfActor`))))
    (`BTFunctionLibrary.SetBlackboardValueAsBool` (`self.bIsWorking`) _canwork)
    (if (not _canwork)
      (`BTFunctionLibrary.SetBlackboardValueAsObject` (`self.TargetToFollow`)))
    (`self.FinishExecute` _canwork)))