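; AI_Character is an agent with Hunger and Sleep needs that destroys itself when either runs out.
; A looping timer set at BeginPlay decays both values, faster while IsWorking is set.
; External events set the work state, apply debuffs, or trigger eating and sleeping, which restore the matching need in fixed steps.
; Note that IsHungry returns true while Hunger is above HungerLimit, although higher Hunger means better fed.
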(event `self.ReceiveActorBeginOverlap`
  (params (OtherActor :type "Actor Object Reference")))

(event `self.ReceiveTick`
  (params (DeltaSeconds :type "Float (single-precision)")))

(event `self.ReceiveBeginPlay`
  ;[1 1 1] Cause Decay
  (`KismetSystemLibrary.K2_SetTimer` self "DecayFunction" (`self.DecayTime`) true))

(event `self.SetIsWorking`
  (params (IsWorking :type Boolean))
  (set `self.bIsWorking` IsWorking))

(event `self.AllowBedForSleep`
  (`self.SleepInBed`))

(event `self.GivePlateToEat`
  (`self.EatFood`))

(event `self.DoHungerDeBuff`
  (params (HungerDebuff :type Integer))
  (set `self.hunger` (- (`self.hunger`) (`KismetMathLibrary.Conv_IntToDouble` HungerDebuff))))

(event `self.DoSleepDeBuff`
  (params (SleepDebuff :type Integer))
  (set `self.sleep` (- (`self.sleep`) (`KismetMathLibrary.Conv_IntToDouble` SleepDebuff))))

(fn `DecayFunction`
  (bind _hunger (`self.hunger`))
  (bind _sleep (`self.sleep`))
  (`|ExecutionSequence`
    (:`then_0`
      ;[0.6539 0.6464 1] Hunger Decay
      (if (> _hunger 0.0)
        (if (`self.bIsWorking`)
          (set `self.hunger` (- _hunger 5.0))
          (else
            (set `self.hunger` (- _hunger 1.0))))
        (else
          (`self.K2_DestroyActor`))))
    (:`then_1`
      ;[0.6539 0.6464 1] Sleep Decay
      (if (> _sleep 0.0)
        (if (`self.bIsWorking`)
          (set `self.sleep` (- _sleep 5.0))
          (else
            (set `self.sleep` (- _sleep 1.0))))
        (else
          (`self.K2_DestroyActor`))))))

(fn `EatFood`
  (if (< (`self.hunger`) 100.0)
    (set `self.hunger` (+ (`self.hunger`) 5.0))
    (`KismetSystemLibrary.PrintString` "Nom Nom!")))

(fn `GetIsWorking`
  (returns (IsWorking :type Boolean))
  (return (`self.bIsWorking`)))

(fn `IsHungry`
  (returns (IsHungry :type Boolean))
  (return (> (`self.hunger`) (`self.hungerLimit`))))

(fn `SleepInBed`
  (bind _sleep (`self.sleep`))
  (if (< _sleep 100.0)
    (set `self.sleep` (+ _sleep 5.0))
    (`KismetSystemLibrary.PrintString` "Zz. Zz.")))

(fn `UserConstructionScript`)