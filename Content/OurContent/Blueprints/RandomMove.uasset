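; RandomMove is a Behavior Tree decorator for AI run by Follower_AI_CON, picking a random position as a side effect of its condition check.
; PerformConditionCheck casts the owner to that controller, caches it, writes GetRandomPoint to the RandomPosition blackboard key, then returns true.
; An unconnected vector calculation for a small random X/Y offset around the controlled pawn remains unused.
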(fn `PerformConditionCheck`
  (params (OwnerActor :type "Actor Object Reference"))
  (returns (ReturnValue :type Boolean))
  (bind _asfollower_ai_con (cast `/Game/OurContent/Blueprints/Follower_AI_CON` OwnerActor))
  (set `self.AI_CON_Ref` _asfollower_ai_con)
  (`BTFunctionLibrary.SetBlackboardValueAsVector` (`self.RandomPosition`) (`NavigationSystem.GetRandomPoint` null))
  (return true))