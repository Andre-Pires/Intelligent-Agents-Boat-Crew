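; Behavior tree task that sends the pawn of a Follower_AI_CON to random navigation points.
; On Tick it caches the controller, then issues AIMoveTo toward a random point within a large radius around a hardcoded X/Y origin at the pawn's current height.
; The move is reissued with a new point each tick, and the task finishes only when a move succeeds, with no failure handling.
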(event `self.ReceiveTick`
  (params (OwnerActor :type "Actor Object Reference") (DeltaSeconds :type "Float (single-precision)"))
  (bind _returnvalue (`Controller.K2_GetPawn` (`self.AI_CON_Ref`)))
  (if (not (!= (`self.AI_CON_Ref`) null))
    (bind _asfollower_ai_con (cast `/Game/OurContent/Blueprints/Follower_AI_CON` OwnerActor))
    (set `self.AI_CON_Ref` _asfollower_ai_con))
  (`|AIMoveTo` _returnvalue (`NavigationSystem.GetRandomPointInRadius` (`KismetMathLibrary.MakeVector` -265.0 0.0 (.z (`Actor.K2_GetActorLocation` _returnvalue))) 50000.0) null 100.0 true
    (:`OnSuccess`
      (`self.FinishExecute` true))))