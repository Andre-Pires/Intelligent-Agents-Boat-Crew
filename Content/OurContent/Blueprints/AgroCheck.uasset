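; AgroCheck is a behavior tree node that picks targets for follower AI by need: food, bed, otherwise machines to work.
; Each tick it sphere-traces around the pawn and filters hits by actor tag.
; A line trace ignoring AI characters confirms visibility, then writes the target and location to the Blackboard or clears the target.
; Sleepiness uses a threshold, while the hunger check always returns false, leaving the food branch inactive.
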(event `self.ReceiveTick`
  (params (OwnerActor :type "Actor Object Reference") (DeltaSeconds :type "Float (single-precision)"))
  (bind _returnvalue (`Actor.K2_GetActorLocation` (`Controller.K2_GetPawn` (`self.AI_CON_Ref`))))
  (if (not (!= (`self.AI_CON_Ref`) null))
    (bind _asfollower_ai_con (cast `/Game/OurContent/Blueprints/Follower_AI_CON` OwnerActor))
    (set `self.AI_CON_Ref` _asfollower_ai_con))
  (bind _outactors (`GameplayStatics.GetAllActorsOfClass` "/Game/OurContent/Blueprints/AI_Character.AI_Character_C"))
  (set `self.MyLocation` _returnvalue)
  (bind _outhits (`KismetSystemLibrary.SphereTraceMultiForObjects` _returnvalue (+ _returnvalue (0.0 0.0 15.0)) 1500.0 (`|MakeArray` "ObjectTypeQuery2" :!type "EngineTypes.EObjectTypeQuery Enum") false _outactors))
  (for _array_element _outhits
    ;[1 1 1] Test if actor is food and we're hungry
    (bind _ishungry (`self.isHungry` (`self.AI_CON_Ref`)))
    (if _ishungry
      (bind (_bblockinghit _time _location _normal _impactpoint _impactnormal _physmat _hitactor) (`GameplayStatics.BreakHitResult` _array_element))
      (if (== _ishungry (`Actor.ActorHasTag` _hitactor (`self.Food`)))
        (bind _outhit (`KismetSystemLibrary.LineTraceSingle` (`self.MyLocation`) (`Actor.K2_GetActorLocation` _hitactor) "TraceTypeQuery2" false _outactors "ForDuration" :!label _label))
        (bind (_bblockinghit_2 _time_2 _location_2 _normal_2 _impactpoint_2 _impactnormal_2 _physmat_2 _hitactor_2) (`GameplayStatics.BreakHitResult` _outhit))
        (if (== _hitactor_2 _hitactor)
          (`BTFunctionLibrary.SetBlackboardValueAsObject` (`self.TargetToFollow`) _hitactor_2)
          (`BTFunctionLibrary.SetBlackboardValueAsVector` (`self.TargetLocation`) (`Actor.K2_GetActorLocation` _hitactor_2))
          (else
            (`BTFunctionLibrary.SetBlackboardValueAsObject` (`self.TargetToFollow`)))))
      (else
        ;[1 1 1] Test if actor is bed and we're sleepy
        (bind _issleepy (`self.isSleepy` (`self.AI_CON_Ref`)))
        (if _issleepy
          (if (== _issleepy (`Actor.ActorHasTag` _hitactor (`self.Bed`)))
            (goto _label))
          (else
            ;[1 1 1] Only then search machines to work
            (if (`Actor.ActorHasTag` _hitactor (`self.Machine`))
              (goto _label))))))))

(fn `isHungry`
  (params (AI_CON_Ref :type "Actor Object Reference"))
  (returns (isHungry :type Boolean))
  (bind _asai_character (cast `/Game/OurContent/Blueprints/AI_Character` AI_CON_Ref))
  (return false))

(fn `isSleepy`
  (params (AI_CON_Ref :type "Actor Object Reference"))
  (returns (isSleepy :type Boolean))
  (bind _asai_character (cast `/Game/OurContent/Blueprints/AI_Character` AI_CON_Ref))
  (return (<= (`/Game/OurContent/Blueprints/AI_Character.sleep` _asai_character) (`self.ThresholdSleep`))))