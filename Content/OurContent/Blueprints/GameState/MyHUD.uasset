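; HUD for a ship game that shows machine resources, distance traveled and the victory or defeat screen with a restart prompt.
; Each DrawHUD polls the GameMode through message calls and draws colored text with DrawText, without widgets.
; Resource readouts are grouped by ship area: cave (engine), deck and kitchen.
; A separate GameOverState function duplicates the end screen at different positions but is not called in this graph.
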(event `self.ReceiveDrawHUD`
  (params (SizeX :type Integer) (SizeY :type Integer))
  (bind _returnvalue (`GameplayStatics.GetGameMode`))
  (`|ExecutionSequence`
    (:`then_1`
      ;[0.7284 1 0.6711] HUD - Barco
      (bind (_currentamountofcoal _currentamountoffire _currentamountofvapor _currentamountofvelocitymotor _currentamountofdirection _currentamountofvelocityleme _currentamountofprovisions _currentamountofuncookedfood _currentamountofcookedfood _currentamountofplates) (message `/Game/OurContent/Blueprints/BPI_Gameplay/BPI_Game_Mode.GetCurrentAmountOfMachineElements` _returnvalue))
      (`|ExecutionSequence`
        (:`then_0`
          ;;[1 0.4443 0.9976] Cave
          (`|ExecutionSequence`
            (:`then_0`
              (`self.DrawText` (`KismetStringLibrary.Concat_StrStr` "Coal:  " (`KismetStringLibrary.Conv_IntToString` _currentamountofcoal)) (struct :`R` 1.0 :`G` 0.45963 :`B` 0.919025 :`A` 1.0) 10.0 150.0))
            (:`then_1`
              (`self.DrawText` (`KismetStringLibrary.Concat_StrStr` "Fire:  " (`KismetStringLibrary.Conv_IntToString` _currentamountoffire)) (struct :`R` 0.705 :`G` 0.301176 :`B` 0.599283 :`A` 1.0) 10.0 170.0))
            (:`then_2`
              (`self.DrawText` (`KismetStringLibrary.Concat_StrStr` "Vapor: " (`KismetStringLibrary.Conv_IntToString` _currentamountofvapor)) (struct :`R` 0.57 :`G` 0.22535 :`B` 0.545784 :`A` 1.0) 10.0 190.0))
            (:`then_3`
              (`self.DrawText` (`KismetStringLibrary.Concat_StrStr` "Velocity Motor:  " (`KismetStringLibrary.Conv_IntToString` _currentamountofvelocitymotor)) (struct :`R` 0.645 :`G` 0.255001 :`B` 0.617598 :`A` 1.0) 10.0 210.0))))
        (:`then_1`
          ;;[0.9843 1 0.6511] Convés
          (`|ExecutionSequence`
            (:`then_0`
              (`self.DrawText` (`KismetStringLibrary.Concat_StrStr` "Direction: " (`KismetStringLibrary.Conv_IntToString` _currentamountofdirection)) (struct :`R` 0.564843 :`G` 0.57 :`B` 0.30979 :`A` 1.0) 10.0 240.0))
            (:`then_1`
              (`self.DrawText` (`KismetStringLibrary.Concat_StrStr` "Velocity Leme:  " (`KismetStringLibrary.Conv_IntToString` _currentamountofvelocityleme)) (struct :`R` 0.645 :`G` 0.582982 :`B` 0.362081 :`A` 1.0) 10.0 260.0))))
        (:`then_2`
          ;;[0.3117 1 0.3016] Cozinha
          (`|ExecutionSequence`
            (:`then_0`
              (`self.DrawText` (`KismetStringLibrary.Concat_StrStr` "Provisions:  " (`KismetStringLibrary.Conv_IntToString` _currentamountofprovisions)) (struct :`R` 0.256697 :`G` 1.0 :`B` 0.299762 :`A` 1.0) 10.0 290.0))
            (:`then_1`
              (`self.DrawText` (`KismetStringLibrary.Concat_StrStr` "Uncooked food: " (`KismetStringLibrary.Conv_IntToString` _currentamountofuncookedfood)) (struct :`R` 0.256697 :`G` 1.0 :`B` 0.299762 :`A` 1.0) 10.0 310.0))
            (:`then_2`
              (`self.DrawText` (`KismetStringLibrary.Concat_StrStr` "Cooked food: " (`KismetStringLibrary.Conv_IntToString` _currentamountofcookedfood)) (struct :`R` 0.256697 :`G` 1.0 :`B` 0.299762 :`A` 1.0) 10.0 330.0))
            (:`then_3`
              (`self.DrawText` (`KismetStringLibrary.Concat_StrStr` "Plates: " (`KismetStringLibrary.Conv_IntToString` _currentamountofplates)) (struct :`R` 0.160435 :`G` 0.625 :`B` 0.187351 :`A` 1.0) 10.0 350.0))))))
    (:`then_2`
      ;;[1 1 1] Distance
      (bind _currentdistancetravelled (message `/Game/OurContent/Blueprints/BPI_Gameplay/BPI_Game_Mode.GetCurrentDistanceTravelled` _returnvalue))
      (`self.DrawText` (`KismetStringLibrary.Concat_StrStr` "Distance Traveled: " (`KismetStringLibrary.Conv_IntToString` _currentdistancetravelled)) (struct :`R` 0.88 :`G` 0.311089 :`B` 0.252171 :`A` 1.0) 10.0 390.0))
    (:`then_3`
      (bind _has_ended (message `/Game/OurContent/Blueprints/BPI_Gameplay/BPI_Game_Mode.HasGameEnded` _returnvalue))
      (if _has_ended
        (bind _has_won (message `/Game/OurContent/Blueprints/BPI_Gameplay/BPI_Game_Mode.HasWon` _returnvalue))
        (if _has_won
          (`self.DrawText` "VICTORY!" (struct :`R` 0.177808 :`G` 1.0 :`B` 0.329294 :`A` 1.0) 130.0 150.0 null 10.0)
          (else
            (`self.DrawText` "DEFEAT!" (struct :`R` 1.0 :`G` 0.279722 :`B` 0.298823 :`A` 1.0) 130.0 150.0 null 10.0)))
        (`self.DrawText` "Press F to restart" (struct :`R` 0.207536 :`G` 0.378636 :`B` 1.0 :`A` 1.0) 130.0 250.0 null 7.0)))))

(fn `GameOverState`
  (params (HasWon :type Boolean :default false))
  (if HasWon
    (`self.DrawText` "VICTORY!" (struct :`R` 0.177808 :`G` 1.0 :`B` 0.329294 :`A` 1.0) 100.0 300.0 null 10.0)
    (else
      (`self.DrawText` "DEFEAT!" (struct :`R` 1.0 :`G` 0.279722 :`B` 0.298823 :`A` 1.0) 10.0 150.0 null 10.0)))
  (`self.DrawText` "Press F to restart" (struct :`R` 0.207536 :`G` 0.378636 :`B` 1.0 :`A` 1.0) 10.0 150.0 null 7.0))

(fn `UserConstructionScript`)