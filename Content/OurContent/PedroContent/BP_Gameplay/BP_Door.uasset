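; BP_Door is a locked door that opens once the player has collected all pickups.
; When the player character overlaps its sphere collider, it asks the game mode whether every pickup has been picked up.
; If so, a timeline moves the door mesh vertically by adding a relative Z offset on each update.
; Otherwise it shows locked text, which a timer hides after a configurable delay.
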(event `self.SphereCollider.OnComponentBeginOverlap`
  (params (OtherActor :type "Actor Object Reference") (OtherComp :type "PrimitiveComponent Object Reference") (OtherBodyIndex :type Integer) (bFromSweep :type Boolean) (SweepResult :type "EngineTypes.HitResult Structure (by ref)"))
  (if (== OtherActor (`GameplayStatics.GetPlayerCharacter` 0))
    (bind _ballpickups_picked_up (message `/Game/TopDownBP/BPI_Gameplay/BPI_Game_Mode.HaveAllPickUpsBeenPickedUp` (`GameplayStatics.GetGameMode`)))
    (if _ballpickups_picked_up
      (bind (_direction _doordropammount) (`Timeline|DoorOpenAnim`)
        (:`Update`
          (`SceneComponent.K2_AddRelativeLocation` (`self.DoorMesh`) (`KismetMathLibrary.MakeVector` 0.0 0.0 _doordropammount) false)))
      (else
        (`SceneComponent.SetHiddenInGame` (`self.DoorLockedText`) false false)
        (`KismetSystemLibrary.K2_SetTimer` self "TurnOffLockedText" (`self.TimeToDisplayLockedText`))))))

(fn `TurnOffLockedText`
  (`SceneComponent.SetHiddenInGame` (`self.DoorLockedText`) true false))

(fn `UserConstructionScript`)