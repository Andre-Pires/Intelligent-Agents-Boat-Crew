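; Base machine Blueprint for a production chain, with a configurable mesh, a stock value and optional timed decay.
; The first actor to overlap its sphere becomes the worker, running a looping work timer until it leaves.
; Each work tick consumes stock and passes produced output to the connected machine's stock.
; Work and decay ticks both report to the game mode by machine type, even when stock is empty.
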(event `self.ReceiveBeginPlay`
  ;[1 1 1] Cause Decay
  (if (`self.bHasDecay`)
    (`KismetSystemLibrary.K2_SetTimer` self "DecayFunction" (`self.DecayTime`) true)))

(event `self.SphereCollider.OnComponentBeginOverlap`
  (params (OtherActor :type "Actor Object Reference") (OtherComp :type "PrimitiveComponent Object Reference") (OtherBodyIndex :type Integer) (bFromSweep :type Boolean) (SweepResult :type "EngineTypes.HitResult Structure (by ref)"))
  ;[1 1 1] Work Machine
  (if (not (`self.bIsWorking`))
    (set `self.WorkingAgent` OtherActor)
    (set `self.bIsWorking` true)
    (`KismetSystemLibrary.K2_SetTimer` self "WorkMachine" (`self.WorkSpeed`) true)))

(event `self.SphereCollider.OnComponentEndOverlap`
  (params (OtherActor :type "Actor Object Reference") (OtherComp :type "PrimitiveComponent Object Reference") (OtherBodyIndex :type Integer))
  ;[1 1 1] Stop Work Machine
  (if (== OtherActor (`self.WorkingAgent`))
    (set `self.bIsWorking` false)
    (`KismetSystemLibrary.K2_ClearTimer` self "WorkMachine")))

(fn `DecayFunction`
  (bind _stock (`self.Stock`))
  (bind _returnvalue (`KismetSystemLibrary.GetDisplayName` self))
  (`|ExecutionSequence`
    (:`then_0`
      ;[0.6539 0.6464 1] Machine Stock Decay Effect
      (if (> _stock 0)
        (set `self.Stock` (- _stock (`self.DecayAmount`)))
        ;[1 1 1] Debugging
        (if (== _returnvalue (`KismetSystemLibrary.GetDisplayName` "/Game/TopDownBP/BP_Gameplay/BP_Machine_Set/BP_Machine_Child_Caldeira.BP_Machine_Child_Caldeira"))
          (`KismetSystemLibrary.PrintString` (`KismetStringLibrary.Concat_StrStr` (`KismetStringLibrary.Concat_StrStr` _returnvalue " Has stock value: ") (`KismetStringLibrary.Conv_IntToString` _stock))))))
    (:`then_1`
      ;[0.6141 1 0.622] Update Game Mode
      (message `/Game/TopDownBP/BPI_Gameplay/BPI_Game_Mode.CauseDecay` (`GameplayStatics.GetGameMode`) (`self.MachineType`) (`self.DecayAmount`)))))

(fn `MachineConnection`
  (params (`Produced Ammount` :type Integer))
  ;[1 1 1] Target Machine Stock Update
  (set `self.Stock` (+ (`self.Stock`) `Produced Ammount`)))

(fn `UserConstructionScript`
  (`StaticMeshComponent.SetStaticMesh` (`self.MachineMesh`) (`self.StaticMeshToDisplay`)))

(fn `WorkMachine`
  (bind _stock (`self.Stock`))
  (bind _consumedamount (`self.ConsumedAmount`))
  (bind _producedamount (`self.ProducedAmount`))
  (`|ExecutionSequence`
    (:`then_0`
      ;[0.628 1 0.6668] Update GameMode
      (message `/Game/TopDownBP/BPI_Gameplay/BPI_Game_Mode.WorkMachine` (`GameplayStatics.GetGameMode`) (`self.MachineType`) _consumedamount _producedamount))
    (:`then_1`
      ;[0.4975 0.5072 1] Update Machine Stocks
      (if (> _stock 0)
        (set `self.Stock` (- _stock _consumedamount))
        (`self.MachineConnection` (`self.ConnectedMachine`) _producedamount)))))