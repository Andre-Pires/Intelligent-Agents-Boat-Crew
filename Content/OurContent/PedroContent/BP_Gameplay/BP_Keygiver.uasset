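; BP_Keygiver is a proximity sign that tells the player how many pink and blue pickups are still needed, or that the door is open.
; When the player enters its collision sphere, it gets pickup totals and collected counts from the Game Mode through message calls and updates two text components.
; The text root shows and rotates each tick to face the player until they leave the sphere.
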(event `self.ReceiveTick`
  (params (DeltaSeconds :type "Float (single-precision)"))
  ;[1 1 1] Rotating Text
  (if (`self.bRotateText`)
    (`SceneComponent.K2_SetWorldRotation` (`self.TextRotateRoot`) (`KismetMathLibrary.MakeRot` (.pitch (`KismetMathLibrary.FindLookAtRotation` (`SceneComponent.K2_GetComponentLocation` (`self.TextRotateRoot`)) (`self.K2_GetActorLocation` (`GameplayStatics.GetPlayerCharacter` 0)))) (.yaw (`KismetMathLibrary.FindLookAtRotation` (`SceneComponent.K2_GetComponentLocation` (`self.TextRotateRoot`)) (`self.K2_GetActorLocation` (`GameplayStatics.GetPlayerCharacter` 0)))) (.roll (`SceneComponent.K2_GetComponentRotation` (`self.TextRotateRoot`)))) false)))

(event `self.CollisionSphere.OnComponentBeginOverlap`
  (params (OtherActor :type "Actor Object Reference") (OtherComp :type "PrimitiveComponent Object Reference") (OtherBodyIndex :type Integer) (bFromSweep :type Boolean) (SweepResult :type "EngineTypes.HitResult Structure (by ref)"))
  (bind _returnvalue (`GameplayStatics.GetGameMode`))
  ;[1 1 1] Text Changes
  (if (== OtherActor (`GameplayStatics.GetPlayerCharacter` 0))
    (set `self.bRotateText` true)
    (bind _ballpickups_picked_up (message `/Game/TopDownBP/BPI_Gameplay/BPI_Game_Mode.HaveAllPickUpsBeenPickedUp` (`GameplayStatics.GetGameMode`)))
    (if _ballpickups_picked_up
      ;[1 1 1] Open Door Text
      (`|ExecutionSequence`
        (:`then_0`
          (`TextRenderComponent.SetText` (`self.BluePicksUpsLeft`) "              Is Open"))
        (:`then_1`
          (`TextRenderComponent.SetText` (`self.PinkPickUpsLeft`) "             The Door"))
        (:`then_2`
          (`SceneComponent.SetHiddenInGame` (`self.TextRotateRoot`) false true :!label _label)))
      (else
        (`|ExecutionSequence`
          (:`then_0`
            (bind (_totalnumberofblueinthelevel _totalnumberofpinkinthelevel) (message `/Game/TopDownBP/BPI_Gameplay/BPI_Game_Mode.GetTotalNumberOfPickUpsInTheLevel` _returnvalue)))
          (:`then_1`
            (bind (_currentbluepickupscollected _currentpinkpickupscollected) (message `/Game/TopDownBP/BPI_Gameplay/BPI_Game_Mode.GetCurrentNumberOfPickUps` _returnvalue)))
          (:`then_2`
            (`|ExecutionSequence`
              (:`then_0`
                (`TextRenderComponent.SetText` (`self.PinkPickUpsLeft`) (`KismetStringLibrary.Concat_StrStr` (`KismetStringLibrary.Concat_StrStr` "Get " (`KismetStringLibrary.Conv_IntToString` (- _totalnumberofpinkinthelevel _currentpinkpickupscollected))) " More Pink Pick Ups")))
              (:`then_1`
                (`TextRenderComponent.SetText` (`self.BluePicksUpsLeft`) (`KismetStringLibrary.Concat_StrStr` (`KismetStringLibrary.Concat_StrStr` "Get " (`KismetStringLibrary.Conv_IntToString` (- _totalnumberofblueinthelevel _currentbluepickupscollected))) " More Blue Pick Ups")))))
          (:`then_3`
            (goto _label)))))))

(event `self.CollisionSphere.OnComponentEndOverlap`
  (params (OtherActor :type "Actor Object Reference") (OtherComp :type "PrimitiveComponent Object Reference") (OtherBodyIndex :type Integer))
  ;[1 1 1] Stop Showing Text
  (if (== OtherActor (`GameplayStatics.GetPlayerCharacter` 0))
    (`SceneComponent.SetHiddenInGame` (`self.TextRotateRoot`) true true)
    (set `self.bRotateText` false)))

(fn `UserConstructionScript`)