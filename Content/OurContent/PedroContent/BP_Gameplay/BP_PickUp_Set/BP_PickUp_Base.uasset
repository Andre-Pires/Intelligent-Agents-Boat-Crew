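; Base pickup actor that spins in the world and is collected when the player character touches it.
; The construction script applies the configurable mesh, and Tick applies a frame-rate-independent yaw rotation at a set rate.
; When the sphere collider overlaps the player, it reports its pickup type to the game mode through CollectedPickUpMessage, then destroys itself.
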(event `self.ReceiveTick`
  (params (DeltaSeconds :type "Float (single-precision)"))
  ;[1 1 1] Rotation
  (`self.K2_AddActorLocalRotation` (`KismetMathLibrary.MakeRot` 0.0 (* DeltaSeconds (`self.Rotation Rate`)))))

(event `self.SphereCollider.OnComponentBeginOverlap`
  (params (OtherActor :type "Actor Object Reference") (OtherComp :type "PrimitiveComponent Object Reference") (OtherBodyIndex :type Integer) (bFromSweep :type Boolean) (SweepResult :type "EngineTypes.HitResult Structure (by ref)"))
  ;[1 1 1] Player Colision
  (if (== OtherActor (`GameplayStatics.GetPlayerCharacter` 0))
    (message `/Game/TopDownBP/BPI_Gameplay/BPI_Game_Mode.CollectedPickUp` (`GameplayStatics.GetGameMode`) (`self.PickupType`))
    (`self.K2_DestroyActor`)))

(fn `UserConstructionScript`
  (`StaticMeshComponent.SetStaticMesh` (`self.PickUpMesh`) (`self.StaticMeshToDisplay`)))